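; Player controller for the F13 game that handles the pause menu and character selection UI.
; The pause input toggles WBP_PauseMenu, switching game pause, input mode and mouse cursor along with it.
; Client_ShowCharcaterSelection waits briefly, then opens WBP_CharacterSelection with Game and UI input if the F13PlayerState has no ChosenRole.
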(event Custom|Client_ShowCharcaterSelection
  (bind _self self)
  (Utilities|FlowControl|Delay 2.0)
  (bind _asf13player_state (Utilities|Casting|CastToF13PlayerState (Variables|Default|GetPlayerState _self)))
  (if (Utilities|Array|IsEmpty (Variables|/Script/F13.F13PlayerState|GetChosenRole _asf13player_state))
    (Development|PrintString "Is Empty")
    (bind _returnvalue (UserInterface|CreateWidget "/Game/UI/WBP_CharacterSelection.WBP_CharacterSelection_C" _self))
    (UserInterface|Viewport|AddtoViewport _returnvalue 0)
    (Input|SetInputModeGameandUI _self _returnvalue "DoNotLock" true false)
    (Variables|Default|SetbShowMouseCursor true)
    (else
      (Development|PrintString "Is not empty"))))

(event Custom|TogglePauseMenu
  (if (Utilities|IsValid (Variables|Default|GetPauseMenuWidget))
    (Widget|RemovefromParent (Variables|Default|GetPauseMenuWidget))
    (bind _returnvalue (Game|SetGamePaused false))
    (Variables|Default|SetbIsPaused _returnvalue)
    (Input|SetInputModeGameOnly self false)
    (Variables|Default|SetbShowMouseCursor false)
    (Variables|Default|SetPauseMenuWidget 0)
    (else
      (Game|SetGamePaused true)
      (Variables|Default|SetbIsPaused false)
      (bind _returnvalue_2 (UserInterface|CreateWidget "/Game/UI/WBP_PauseMenu.WBP_PauseMenu_C"))
      (bind _output_get (Variables|Default|SetPauseMenuWidget _returnvalue_2))
      (UserInterface|Viewport|AddtoViewport _output_get 0)
      (Input|SetInputModeUIOnly self _output_get "DoNotLock" false)
      (Variables|Default|SetbShowMouseCursor true))))

(event Input|EnhancedActionEvents|EnhancedInputActionIA_Pause
  (params (ActionValue :type Boolean) (ElapsedSeconds :type Float%20%28double-precision%29) (TriggeredSeconds :type Float%20%28double-precision%29) (InputAction :type Input%20Action%20Object%20Reference :default "/Game/Characters/Input/IA_Pause.IA_Pause"))
  (CallFunction|TogglePauseMenu))

(event EventBeginPlay)

(event EventTick
  (params (DeltaSeconds :type Float%20%28single-precision%29)))

(fn ConstructionScript)