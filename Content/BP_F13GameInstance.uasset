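; BP_F13GameInstance is a game instance Blueprint that handles HMS reconnect and rehost events for multiplayer sessions.
; Reconnect runs an "open" console command built from the stored reconnect address.
; Rehost destroys the current session, then creates a new one with the current LAN setting whether or not that succeeds.
; On successful creation, it opens the level named in the rehost save as a listen server.
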(event EventHMSRehostGame
  (bind _returnvalue (Game|GetPlayerController 0))
  (|DestroySession _returnvalue
    (:OnSuccess
      _)
    (:OnFailure
      _))
  (|Session _returnvalue 0 (Variables|Default|GetCurrentIsLAN) true
    (:OnSuccess
      (Game|OpenLevel(byName) (Utilities|String|StringToName (Utilities|Struct|BreakHMS_GameSave (Variables|Default|GetHMS_RehostGameSave))) true "listen"))))

(event EventHMSReconnecttoGame
  (Development|ExecuteConsoleCommand (Utilities|String|Append "open" (Variables|/Script/HostMigrationSystem.HMS_GameInstance|GetHMS_ReconnectAddress (Class|HMSFunctionLibrary|HMSGetGameInstance))) (Game|GetPlayerController 0)))