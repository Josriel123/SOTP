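; Game instance Blueprint that handles session teardown, reconnecting and rehosting for multiplayer games.
; Shutdown destroys the session, and reconnect runs an open console command built from the address stored on the HMS game instance.
; Rehost destroys any session, then creates a ten-connection LAN session whether or not that succeeded.
; On success it opens the level named in the rehost save as a listen server, with on-screen debug prints.
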(event EventHMSRehostGame
  (bind _returnvalue (Game|GetPlayerController 0))
  (|DestroySession _returnvalue
    (:OnSuccess
      _)
    (:OnFailure
      _))
  (|Session _returnvalue 10 true true
    (:OnSuccess
      (bind _ashms_game_instance (Utilities|Casting|CastToHMS_GameInstance (Game|GetGameInstance)))
      (Development|PrintString (.LevelName (Utilities|Struct|BreakHMS_GameSave (Variables|/Script/HostMigrationSystem.HMS_GameInstance|GetHMS_RehostGameSave _ashms_game_instance))) true true "(R=0.000000,G=0.660000,B=1.000000,A=1.000000)" 5.0)
      (Game|OpenLevel(byName) (Utilities|String|StringToName (.LevelName (Utilities|Struct|BreakHMS_GameSave (Variables|/Script/HostMigrationSystem.HMS_GameInstance|GetHMS_RehostGameSave _ashms_game_instance)))) true "listen")
      (Development|PrintString "Rehosted" true true "(R=0.124906,G=1.000000,B=0.000000,A=1.000000)" 5.0))
    (:OnFailure
      (Development|PrintString "Did not create session"))))

(event EventHMSReconnecttoGame
  (bind _returnvalue (Class|HMSFunctionLibrary|HMSGetGameInstance))
  (bind _hms_reconnectaddress (Variables|/Script/HostMigrationSystem.HMS_GameInstance|GetHMS_ReconnectAddress _returnvalue))
  (Development|ExecuteConsoleCommand (Utilities|String|Append "open " _hms_reconnectaddress) 0)
  (Development|PrintString _hms_reconnectaddress))

(event EventShutdown
  (|DestroySession))