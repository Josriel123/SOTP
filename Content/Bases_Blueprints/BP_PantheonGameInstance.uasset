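; Game instance that handles online session cleanup and host migration through an HMS system.
; Shutdown destroys the session, and the reconnect event sends clients to the new host's address with an open console command.
; On rehost, it replaces the old session with a LAN one, deserializes the HMS save buffers into a new game save object, then reopens the saved level as a listen server flagged for rehosting.
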(event EventHMSRehostGame
  (bind _returnvalue (Game|GetPlayerController 0))
  ;[0.15 0.15 0.15 0.5] New Host Creates New Session
  (|DestroySession _returnvalue
    (:OnSuccess
      _)
    (:OnFailure
      _))
  (|Session _returnvalue 10 true true
    (:OnSuccess
      (bind _ashms_game_instance (Utilities|Casting|CastToHMS_GameInstance (Game|GetGameInstance)))
      (bind _returnvalue_2 (Game|ConstructObjectfromClass "/Game/Bases_Blueprints/BP_HMSGameSave.BP_HMSGameSave_C"))
      (bind _output_get (Variables|Default|SetBP_HMSGameSave _returnvalue_2))
      (Class|HMSFunctionLibrary|HMSDeserializeObjectProperties _output_get (.CustomGameSaveDataObjectPropertyBuffers (Utilities|Struct|BreakHMS_GameSave (Variables|/Script/HostMigrationSystem.HMS_GameInstance|GetHMS_RehostGameSave _ashms_game_instance))) true)
      (Game|OpenLevel(byName) (Utilities|String|StringToName (.LevelName (Utilities|Struct|BreakHMS_GameSave (Variables|/Script/HostMigrationSystem.HMS_GameInstance|GetHMS_RehostGameSave _ashms_game_instance)))) true "listen?hms_rehost=1")
      (Utilities|IsValid (Variables|Default|GetBP_HMSGameSave)
        (:Is%20Valid
          (Development|PrintString "GameSave valid")
          (Development|PrintString "Rehosted" true true "(R=0.124906,G=1.000000,B=0.000000,A=1.000000)" 5.0))
        (:Is%20Not%20Valid
          (Development|PrintString "GameSave not valid"))))))

(event EventHMSReconnecttoGame
  ;[0.15 0.15 0.15 0.5] Reconnect client to new host
  (Development|ExecuteConsoleCommand (Utilities|String|Append "open " (Variables|/Script/HostMigrationSystem.HMS_GameInstance|GetHMS_ReconnectAddress (Class|HMSFunctionLibrary|HMSGetGameInstance))) 0))

(event EventShutdown
  ;[0.15 0.15 0.15 0.5] Destroys session when closing the window
  (|DestroySession))