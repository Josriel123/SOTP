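; BP_PantheonGameMode is a game mode that handles HMS save and rehost events and keeps a bot counter.
; When a save task starts, SaveGame writes the human player count to the HMS save object and prints it.
; The count skips bot player states and is only computed while no save object is cached.
; Rehosting is handed to C++, and the player-change and character-selection chains are left unconnected.
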(event EventTick
  (params (DeltaSeconds :type Float%20%28single-precision%29)))

(event EventPostLogin
  (params (NewPlayer :type Player%20Controller%20Object%20Reference)))

(event EventHMSonGameRehosted
  (Class|PantheonGameMode|HMSonGameRehostedCpp))

(event EventHMSonCreateGameSaveTaskStarted
  (CallFunction|SaveGame))

(event EventBeginPlay)

(fn ConstructionScript)

(fn SaveGame
  (Utilities|IsValid (Variables|Default|GetBP_HMSGameSave)
    (:Is%20Valid
      _)
    (:Is%20Not%20Valid
      (bind _asbp_hmsgame_save (Utilities|Casting|CastToBP_HMSGameSave (Variables|Default|GetHMS_CustomGameSaveDataObject)))
      (Variables|Default|SetBP_HMSGameSave _asbp_hmsgame_save)
      (for _array_element (Variables|/Script/Engine.GameStateBase|GetPlayerArray (Game|GetGameState))
        (bind _aspantheon_player_state (Utilities|Casting|CastToPantheonPlayerState _array_element))
        (Utilities|IsValid _aspantheon_player_state
          (:Is%20Valid
            (if (not (Variables|/Script/Pantheon.PantheonPlayerState|GetbIsBot _aspantheon_player_state))
              (Variables|Default|SetHumansOnly (+ 1 (Variables|Default|GetHumansOnly)))))))))
  (bind _output_get (Variables|/Game/Bases_Blueprints/BP_HMSGameSave.BP_HMSGameSave_C|SetNumHumans (Variables|Default|GetBP_HMSGameSave) (Variables|Default|GetHumansOnly)))
  (Development|PrintString (Utilities|String|BuildString(Integer) "" "Number of Players: " _output_get)))

(fn GetNextBotIndex
  (Variables|Default|SetBotCounter (+ (Variables|Default|GetBotCounter) 1)))