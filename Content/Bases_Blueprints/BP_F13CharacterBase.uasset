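; Base character Blueprint wired to HMS host migration, showing a Host/Client player ID label on front and back widgets.
; On authority, BeginPlay assigns a random ID unless the game is rehosted without its last save loaded.
; Possessed flags the host from local control on authority, and Tick pushes the prefixed ID into both widgets.
; HMS pre-save and post-load interface events are empty stubs, with transform save/restore nodes left unconnected.
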(event HMSPreSaveActor(HMS_Interface))

(event HMSPostLoadActor(HMS_Interface))

(event EventBeginPlay
  (Networking|SwitchHasAuthority
    (:Authority
      (bind _ashms_game_mode (Utilities|Casting|CastToHMS_GameMode (Game|GetGameMode)))
      (if (.IsGameRehosted (Utilities|Struct|BreakHMS_MigrationFlags (Variables|/Script/HostMigrationSystem.HMS_GameMode|GetHMS_MigrationFlags _ashms_game_mode)))
        (if (.IsLastSaveLoaded (Utilities|Struct|BreakHMS_MigrationFlags (Variables|/Script/HostMigrationSystem.HMS_GameMode|GetHMS_MigrationFlags _ashms_game_mode)))
          (Utilities|FlowControl|Sequence :!label _label
            (:then_1
              (Variables|Default|SetHMS_PlayerIDString (Utilities|String|ToString(Integer) (Math|Random|RandomInteger 1000))))))
        (else
          (goto _label))))))

(event EventPossessed
  (params (NewController :type Controller%20Object%20Reference))
  (Networking|SwitchHasAuthority
    (:Authority
      (Variables|Default|SetHMS_IsHost (Pawn|IsLocallyControlled)))))

(event EventTick
  (params (DeltaSeconds :type Float%20%28single-precision%29))
  (bind _hms_playeridstring (Variables|Default|GetHMS_PlayerIDString))
  (bind _hms_ishost (Variables|Default|GetHMS_IsHost))
  (bind _returnvalue (select _hms_ishost "Host_" "Client_"))
  (bind _returnvalue_2 (Utilities|String|Append _returnvalue _hms_playeridstring))
  (Utilities|FlowControl|Sequence
    (:then_0
      (bind _ashms_w_player_id (Utilities|Casting|CastToHMS_W_PlayerID (UserInterface|GetUserWidgetObject (Variables|Default|GetPlayerIDWidget_Back))))
      (Variables|/Game/UI/HMS_W_PlayerID.HMS_W_PlayerID_C|SetPlayerIDString _ashms_w_player_id _returnvalue_2))
    (:then_1
      (bind _ashms_w_player_id_2 (Utilities|Casting|CastToHMS_W_PlayerID (UserInterface|GetUserWidgetObject (Variables|Default|GetPlayerIDWidget_Front))))
      (Variables|/Game/UI/HMS_W_PlayerID.HMS_W_PlayerID_C|SetPlayerIDString _ashms_w_player_id_2 _returnvalue_2))))

(fn ConstructionScript)