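; BP_F13PlayerController is a player controller that handles menus, cursor and input mode, and being kicked from a session.
; IA_Pause creates or removes the pause menu widget, switching between UI-only and game-only input.
; ShowLobbyUI opens the host lobby menu with UI focus.
; OC_KickPlayer opens MainMenu and destroys the session; a separate cursor toggle event has no active caller here.
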(event Custom|OC_KickPlayer
  (Game|OpenLevel(byName) "MainMenu")
  (|DestroySession
    (:OnSuccess
      (Development|PrintString "Got Kicked" true true "(R=0.255456,G=1.000000,B=0.000000,A=1.000000)" 5.0))))

(event Custom|TogglePauseMenu
  (if (Utilities|IsValid (Variables|Default|GetPauseMenuWidget))
    (Widget|RemovefromParent (Variables|Default|GetPauseMenuWidget))
    (Input|SetInputModeGameOnly self false)
    (Variables|Default|SetbShowMouseCursor false)
    (Variables|Default|SetPauseMenuWidget 0)
    (else
      (bind _returnvalue (UserInterface|CreateWidget "/Game/UI/MainMenu/WBP_PauseMenu.WBP_PauseMenu_C"))
      (bind _output_get (Variables|Default|SetPauseMenuWidget _returnvalue))
      (UserInterface|Viewport|AddtoViewport _output_get 0)
      (Input|SetInputModeUIOnly self _output_get "DoNotLock" false)
      (Variables|Default|SetbShowMouseCursor true))))

(event Custom|ShowLobbyUI
  (bind _returnvalue (Game|GetPlayerController 0))
  (bind _returnvalue_2 (UserInterface|CreateWidget "/Game/UI/Lobby/WBP_HostLobbyMenu.WBP_HostLobbyMenu_C"))
  (UserInterface|Viewport|AddtoViewport _returnvalue_2 0)
  (Input|SetInputModeUIOnly _returnvalue _returnvalue_2 "DoNotLock" false)
  (Variables|/Script/Engine.PlayerController|SetbShowMouseCursor _returnvalue true)
  (Development|PrintString "Showing Lobby UI" true true "(R=0.120546,G=1.000000,B=0.000000,A=1.000000)" 5.0))

(event Custom|ToggleMouse%20Cursor
  (bind _self self)
  (bind _self_2 self)
  (if (Variables|Default|GetbMouseCursorShown)
    (Variables|Default|SetbMouseCursorShown false)
    (Input|SetInputModeGameOnly _self_2 false)
    (Variables|Default|SetbShowMouseCursor _self_2 false)
    (else
      (Variables|Default|SetbMouseCursorShown true)
      (Input|SetInputModeUIOnly _self 0 "DoNotLock" false)
      (Variables|Default|SetbShowMouseCursor _self true))))

(event Input|EnhancedActionEvents|EnhancedInputActionIA_Pause
  (params (ActionValue :type Boolean) (ElapsedSeconds :type Float%20%28double-precision%29) (TriggeredSeconds :type Float%20%28double-precision%29) (InputAction :type Input%20Action%20Object%20Reference :default "/Game/Characters/Input/IA_Pause.IA_Pause"))
  (CallFunction|TogglePauseMenu))

(event EventBeginPlay
  (|CallParentFunction))

(event Input|KeyboardEvents|H
  (params (Key :type Key%20Structure :default "None")))

(fn ConstructionScript)