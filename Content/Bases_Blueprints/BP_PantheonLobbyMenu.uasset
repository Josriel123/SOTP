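; BP_PantheonLobbyMenu is the lobby game mode, showing the lobby UI to each player who logs in.
; ServerStartMatch checks every PlayerState is ready, then server-travels to ThirdPersonMap as a listen server, passing human and bot counts as URL options and switching the first controller to game input.
; KickPlayer indexes AllPlayerControllers to trigger a kick, but the node that adds to an array is unconnected.
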(event Custom|ServerStartMatch
  (bind _returnvalue (Game|GetPlayerController 0))
  (bind _array_element (Utilities|Array|ForEachLoopwithBreak (Variables|/Script/Engine.GameStateBase|GetPlayerArray (Game|GetGameState)) :!label _label)
    (:LoopBody
      (bind _aspantheon_player_state (Utilities|Casting|CastToPantheonPlayerState _array_element))
      (if (Class|PantheonPlayerState|IsReady _aspantheon_player_state)
        (Variables|Default|SetAllReady true)
        (else
          (Variables|Default|SetAllReady false)
          (Development|PrintString "Someone is not ready")
          (goto _label Break))))
    (:Completed
      (if (Variables|Default|GetAllReady)
        (bind _output_get (Variables|Default|SetHumanCount (Utilities|Array|Length (Variables|/Script/Engine.GameStateBase|GetPlayerArray (Game|GetGameState)))))
        (Class|AdvancedSessionsLibrary|ServerTravel (Utilities|String|BuildString(Integer) (Utilities|String|BuildString(Integer) "" "/Game/ThirdPerson/Maps/ThirdPersonMap?listen?humans=" _output_get) "?bots=" (Variables|Default|GetbBots)) true false)
        (Input|SetInputModeGameOnly _returnvalue false)
        (Variables|/Script/Engine.PlayerController|SetbShowMouseCursor _returnvalue false)))))

(event EventPostLogin
  (params (NewPlayer :type Player%20Controller%20Object%20Reference))
  (bind _asbp_pantheon_player_controller (Utilities|Casting|CastToBP_PantheonPlayerController NewPlayer))
  (Default|ShowLobbyUI _asbp_pantheon_player_controller))

(event EventOnLogout
  (params (ExitingController :type Controller%20Object%20Reference)))

(fn ConstructionScript)

(fn KickPlayer
  (params (PlayerID :type Integer))
  (Default|OCKickPlayer (Utilities|Array|Get(acopy) (Variables|Default|GetAllPlayerControllers) PlayerID)))