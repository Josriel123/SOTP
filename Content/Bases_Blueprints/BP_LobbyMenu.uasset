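; Lobby game mode for an F13 multiplayer game that tracks joining and leaving players and starts the match.
; Login and logout update the controller list and, after a short delay, refresh the game state's player list; new players also get the lobby UI.
; Match start checks every player is ready, then server-travels to the third-person map with human and bot counts as URL options.
; Players can be kicked by controller list index.
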(event Custom|ServerStartMatch
  (bind _returnvalue (Game|GetPlayerController 0))
  (bind _array_element (Utilities|Array|ForEachLoopwithBreak (Variables|/Script/Engine.GameStateBase|GetPlayerArray (Game|GetGameState)) :!label _label)
    (:LoopBody
      (bind _asf13player_state (Utilities|Casting|CastToF13PlayerState _array_element))
      (if (Class|F13PlayerState|IsReady _asf13player_state)
        (Variables|Default|SetAllReady true)
        (else
          (Variables|Default|SetAllReady false)
          (Development|PrintString "Someone is not ready")
          (goto _label Break))))
    (:Completed
      (if (Variables|Default|GetAllReady)
        (bind _output_get (Variables|Default|SetHumanCount (Utilities|Array|Length (Variables|/Script/Engine.GameStateBase|GetPlayerArray (Game|GetGameState)))))
        (Class|AdvancedSessionsLibrary|ServerTravel (Utilities|String|BuildString(Integer) (Utilities|String|BuildString(Integer) "" "/Game/ThirdPerson/Maps/ThirdPersonMap?listen?humans=" _output_get) "?bots=" (Variables|Default|GetbBots)) true false)
        (Input|SetInputModeGameOnly _returnvalue false)
        (Variables|/Script/Engine.PlayerController|SetbShowMouseCursor _returnvalue false)))))

(event Custom|UpdatePlayerList
  (Utilities|FlowControl|Delay 0.3)
  (bind _asbp_f13game_state (Utilities|Casting|CastToBP_F13GameState (Game|GetGameState)))
  (Default|UpdatePlayerList _asbp_f13game_state))

(event EventPostLogin
  (params (NewPlayer :type Player%20Controller%20Object%20Reference))
  (bind _asbp_f13player_controller (Utilities|Casting|CastToBP_F13PlayerController NewPlayer))
  (Utilities|Array|Add (Variables|Default|GetAllPlayerControllers) _asbp_f13player_controller)
  (Default|ShowLobbyUI _asbp_f13player_controller)
  (CallFunction|UpdatePlayerList))

(event EventOnLogout
  (params (ExitingController :type Controller%20Object%20Reference))
  (bind _asbp_f13player_controller (Utilities|Casting|CastToBP_F13PlayerController ExitingController))
  (Utilities|Array|RemoveItem (Variables|Default|GetAllPlayerControllers) _asbp_f13player_controller)
  (CallFunction|UpdatePlayerList))

(fn ConstructionScript)

(fn KickPlayer
  (params (PlayerID :type Integer))
  (Default|OCKickPlayer (Utilities|Array|Get(acopy) (Variables|Default|GetAllPlayerControllers) PlayerID)))