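; Base character Blueprint that gives players and bots a replicated name tag shown on front and back nameplate widgets.
; On possess and unpossess, the authority builds NameTag from the player name plus a Host or Client suffix, or a numbered bot name via BP_PantheonGameMode.
; OnRep_NameTag refreshes both widgets' text, while Tick also copies the string into them every frame.
; HMS save/load interface events are empty stubs.
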(event HMSPreSaveActor(HMS_Interface))

(event HMSPostLoadActor(HMS_Interface))

(event EventUnpossessed
  (params (OldController :type Controller%20Object%20Reference))
  (if (Ability|HasAuthority OldController)
    (CallFunction|BuildandSetNameTag)))

(event EventPossessed
  (params (NewController :type Controller%20Object%20Reference))
  (if (Ability|HasAuthority NewController)
    (CallFunction|BuildandSetNameTag)))

(event EventTick
  (params (DeltaSeconds :type Float%20%28single-precision%29))
  (bind _nametag (Variables|Default|GetNameTag))
  (Utilities|FlowControl|Sequence
    (:then_0
      (bind _ashms_w_player_id (Utilities|Casting|CastToHMS_W_PlayerID (UserInterface|GetUserWidgetObject (Variables|Default|GetPlayerIDWidget_Back))))
      (Variables|/Game/UI/HMS_W_PlayerID.HMS_W_PlayerID_C|SetPlayerIDString _ashms_w_player_id _nametag))
    (:then_1
      (bind _ashms_w_player_id_2 (Utilities|Casting|CastToHMS_W_PlayerID (UserInterface|GetUserWidgetObject (Variables|Default|GetPlayerIDWidget_Front))))
      (Variables|/Game/UI/HMS_W_PlayerID.HMS_W_PlayerID_C|SetPlayerIDString _ashms_w_player_id_2 _nametag))))

(fn ConstructionScript)

(fn OnRepNameTag
  (CallFunction|UpdateNamePlate))

(fn UpdateNamePlate
  (Utilities|FlowControl|Sequence
    (:then_0
      (bind _ashms_w_player_id (Utilities|Casting|CastToHMS_W_PlayerID (UserInterface|GetUserWidgetObject (Variables|Default|GetPlayerIDWidget_Front))))
      (Variables|/Game/UI/HMS_W_PlayerID.HMS_W_PlayerID_C|SetPlayerIDString _ashms_w_player_id (Variables|Default|GetNameTag))
      (Default|SetNameText _ashms_w_player_id (Utilities|Text|ToText(String) (Variables|Default|GetNameTag))))
    (:then_1
      (bind _ashms_w_player_id_2 (Utilities|Casting|CastToHMS_W_PlayerID (UserInterface|GetUserWidgetObject (Variables|Default|GetPlayerIDWidget_Back))))
      (Variables|/Game/UI/HMS_W_PlayerID.HMS_W_PlayerID_C|SetPlayerIDString _ashms_w_player_id_2 (Variables|Default|GetNameTag))
      (Default|SetNameText _ashms_w_player_id_2 (Utilities|Text|ToText(String) (Variables|Default|GetNameTag))))))

(fn BuildandSetNameTag
  (bind _returnvalue (Pawn|IsPlayerControlled))
  (Networking|SwitchHasAuthority
    (:Authority
      (if _returnvalue
        (bind _asplayer_controller (Utilities|Casting|CastToPlayerController (Pawn|GetController)))
        (bind _output_get (Variables|Default|SetbIsHost (Pawn|IsLocalController _asplayer_controller)))
        (if _output_get
          (Variables|Default|SetNameTag (Utilities|String|Append (PlayerState|GetPlayerName (Variables|/Script/Engine.Controller|GetPlayerState _asplayer_controller)) " (Host)"))
          (else
            (Variables|Default|SetNameTag (Utilities|String|Append (PlayerState|GetPlayerName (Variables|/Script/Engine.Controller|GetPlayerState _asplayer_controller)) " (Client)"))))
        (else
          (Variables|Default|SetbIsBot _returnvalue)
          (bind _asbp_pantheon_game_mode (Utilities|Casting|CastToBP_PantheonGameMode (Game|GetGameMode)))
          (Default|GetNextBotIndex _asbp_pantheon_game_mode)
          (Variables|Default|SetNameTag (Utilities|String|BuildString(Integer) "" "Bot " (Variables|/Game/Bases_Blueprints/BP_PantheonGameMode.BP_PantheonGameMode_C|GetBotCounter _asbp_pantheon_game_mode))))))))